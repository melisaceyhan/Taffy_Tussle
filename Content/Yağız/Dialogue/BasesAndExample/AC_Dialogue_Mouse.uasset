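; Example dialogue component for a Mouse NPC who asks the player for cheese.
; Overrides Dialogue, branching on tree index and nesting AddDialogue calls whose Pass Through state and chosen option drive the next line.
; Giving cheese switches to a second tree with a random thanks line.
; Other endings clear or partly rewind progress and close the conversation; the first line's Updated state prints a debug string.
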(fn `Dialogue`
  (`parent.Dialogue`)
  (switch `int` (`self.DialogueTreeIndex`)
    (:`0`
      (bind (_state _optionindex) (`self.AddDialogue` "Mouse" "Hi, do you have any cheese?" (`|MakeArray` "Yes" "No" :!type "Text")))
      (switch `/Game/Yağız/Dialogue/Enum_DialogueState` _state
        (:`NewEnumerator0`
          (switch `int` _optionindex
            (:`0`
              (bind (_state_2 _optionindex_2) (`self.AddDialogue` "Mouse" "Great news, can i have some?" (`|MakeArray` "Give Cheese" "Keep Cheese" :!type "Text")))
              (switch `/Game/Yağız/Dialogue/Enum_DialogueState` _state_2
                (:`NewEnumerator0`
                  (switch `int` _optionindex_2
                    (:`0`
                      (bind _state_3 (`self.AddDialogue` "Mouse" "Thank you, you are so kind!" (`|MakeArray` "Continue" :!type "Text")))
                      (switch `/Game/Yağız/Dialogue/Enum_DialogueState` _state_3
                        (:`NewEnumerator0`
                          (`self.SetDialogueTreeIndex` 1))))
                    (:`1`
                      (bind _state_4 (`self.AddDialogue` "Mouse" "You are mean!" (`|MakeArray` "Continue" :!type "Text")))
                      (switch `/Game/Yağız/Dialogue/Enum_DialogueState` _state_4
                        (:`NewEnumerator0`
                          (`self.RemoveDialogueProgress` 2)
                          (`self.CloseConversation`))))))))
            (:`1`
              (bind _state_5 (`self.AddDialogue` "Mouse" "Damn, i really wanted some." (`|MakeArray` "Continue" :!type "Text")))
              (switch `/Game/Yağız/Dialogue/Enum_DialogueState` _state_5
                (:`NewEnumerator0`
                  (`self.ClearDialogueProgress`)
                  (`self.CloseConversation`))))))
        (:`NewEnumerator1`
          (`KismetSystemLibrary.PrintString` "Hello"))))
    (:`1`
      (bind _state_6 (`self.AddDialogue` "Mouse" (`KismetArrayLibrary.Array_Random` (`|MakeArray` "Thanks again" "So good" "You are the man" :!type "Text")) (`|MakeArray` "Continue" :!type "Text")))
      (switch `/Game/Yağız/Dialogue/Enum_DialogueState` _state_6
        (:`NewEnumerator0`
          (`self.ClearDialogueProgress`)
          (`self.CloseConversation`))))))